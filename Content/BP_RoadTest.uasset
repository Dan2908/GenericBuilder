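; BP_RoadTest is a test road actor that snaps a spline to the ground and builds meshes along it.
; The construction script moves each spline point to the hit of a vertical line trace from 5000 units above to 5000 below, keeping its position on a miss.
; DrawMeshes then adds a spline mesh component per segment, using the local locations and tangents of neighbouring points.
; All logic runs in construction, with debug trace drawing and index logging.
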(event EventBeginPlay)

(event Collision|EventActorBeginOverlap
  (params (OtherActor :type Actor%20Object%20Reference)))

(event EventTick
  (params (DeltaSeconds :type Float%20%28single-precision%29)))

(fn ConstructionScript
  (for _index (range 0 (- (Spline|GetNumberOfSplinePoints (Variables|Default|GetSpline)) 1))
    (CallFunction|AttachtoGround _index)
    (Utilities|String|LogString (Utilities|String|Append "Attached index " (Utilities|String|ToString(Integer) _index))))
  (CallFunction|DrawMeshes))

(fn TraceGround
  (params (SplineLocation :type Vector))
  (bind (_outhit _returnvalue) (Collision|LineTraceByChannel (+ SplineLocation "0.000000,0.000000,5000.000000") (+ SplineLocation "0.000000,0.000000,-5000.000000") "TraceTypeQuery3" false 0 "ForDuration"))
  (if _returnvalue
    (return (.location _outhit))
    (else
      (return SplineLocation))))

(fn DrawMeshes
  (bind _spline (Variables|Default|GetSpline))
  (for _index (range 0 (- (Spline|GetNumberOfSplinePoints (Variables|Default|GetSpline)) 2))
    (bind _returnvalue (AddComponent|AddSplineMeshComponent false))
    (SplineMesh|SetStartandEnd _returnvalue (.Location (Spline|GetLocationandTangentatSplinePoint _spline _index "Local")) (.Tangent (Spline|GetLocationandTangentatSplinePoint _spline _index "Local")) (.Location (Spline|GetLocationandTangentatSplinePoint _spline (+ _index 1) "Local")) (.Tangent (Spline|GetLocationandTangentatSplinePoint _spline (+ _index 1) "Local")) true :!class /Script/Engine.SplineMeshComponent)
    (Transformation|AttachComponentToComponent _returnvalue 0 "None" "KeepRelative" "KeepRelative" "KeepRelative" true)))

(fn AttachtoGround
  (params (Index :type Integer))
  (bind _spline (Variables|Default|GetSpline))
  (Spline|SetLocationatSplinePoint _spline Index (CallFunction|TraceGround (Spline|GetLocationatSplinePoint _spline Index "World")) "World" true))